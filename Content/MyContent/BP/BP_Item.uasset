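; BP_Item is an item pickup actor that shows an equip prompt when the player character overlaps it.
; On overlap it sets IsOverlappingItem on XBotCharacter and creates a UI_EquipItem widget, passing it to SetCorrectItemName before adding it to the viewport.
; End overlap clears the flag and removes every top-level UI_EquipItem widget.
; SetCorrectItemName is empty here, so this Blueprint itself sets no item name.
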(event `self.ReceiveActorBeginOverlap`
  (params (OtherActor :type "Actor Object Reference"))
  (bind _asxbot_character (cast `XBotCharacter` OtherActor))
  (set `XBotCharacter.IsOverlappingItem` true _asxbot_character)
  (bind _returnvalue (`|CreateWidget` "/Game/MyContent/BP/UI_EquipItem.UI_EquipItem_C"))
  (`self.SetCorrectItemName` _returnvalue)
  (`UserWidget.AddToViewport` _returnvalue 0))

(event `self.ReceiveActorEndOverlap`
  (params (OtherActor :type "Actor Object Reference"))
  (bind _asxbot_character (cast `XBotCharacter` OtherActor))
  (set `XBotCharacter.IsOverlappingItem` false _asxbot_character)
  (bind _foundwidgets (`WidgetBlueprintLibrary.GetAllWidgetsOfClass` "/Game/MyContent/BP/UI_EquipItem.UI_EquipItem_C"))
  (for _array_element _foundwidgets
    (`Widget.RemoveFromParent` _array_element)))

(fn `SetCorrectItemName`
  (params (NewParam :type "/Game/MyContent/BP/UI_EquipItem Object Reference")))

(fn `UserConstructionScript`)