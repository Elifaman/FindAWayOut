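; AI controller for the bot that runs BT_AIBot on BB_AIBot and tracks the player through AI Perception.
; Sensing player character 0 writes it to the blackboard key "TargerActor" (spelled as such), sets focus on it and cancels any pending lose-target timer.
; Losing perception starts a short grace timer that clears the key and focus when it expires, so brief breaks in sensing keep the target.
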(event `self.AIPerception.OnTargetPerceptionUpdated`
  (params (Actor :type "Actor Object Reference") (Stimulus :type "AIStimulus Structure"))
  (set `self.SensedActor` Actor)
  (if (== Actor (`GameplayStatics.GetPlayerCharacter` 0))
    (if (`.bSuccessfullySensed` (break `AIStimulus` Stimulus))
      (`BlackboardComponent.SetValueAsObject` (`self.Blackboard`) "TargerActor" (`self.SensedActor`))
      (`self.K2_SetFocus` (`self.SensedActor`))
      (`KismetSystemLibrary.K2_ClearAndInvalidateTimerHandle` (`self.LoseTargetTimer`))
      (else
        (bind _returnvalue (`KismetSystemLibrary.K2_SetTimerDelegate` (delegate `LoseTarget`) 3.0))
        (set `self.LoseTargetTimer` _returnvalue)))))

(event `LoseTarget`
  (`BlackboardComponent.SetValueAsObject` (`self.Blackboard`) "TargerActor" null)
  (`self.K2_ClearFocus`))

(event `self.ReceiveBeginPlay`
  (`self.UseBlackboard` "/Game/MyContent/AI/Bot/BB_AIBot.BB_AIBot")
  (`self.RunBehaviorTree` "/Game/MyContent/AI/Bot/BT_AIBot.BT_AIBot"))

(fn `UserConstructionScript`)