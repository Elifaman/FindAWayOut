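; BP_AIEnemy is an AI enemy actor that carries a gun and shoots at a given target.
; On BeginPlay it snaps its gun mesh to the body mesh's weapon socket.
; ShootEnemy spawns a muzzle emitter at the gun socket, then runs a visibility line trace from the actor to the target.
; Damage is applied only when the trace hits that target directly.
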(event `ShootEnemy`
  (params (EnemyToShoot :type "Actor Object Reference"))
  (`self.PlayShootFX`)
  (bind (_outhit _returnvalue) (`KismetSystemLibrary.LineTraceSingle` (`self.K2_GetActorLocation`) (`self.K2_GetActorLocation` EnemyToShoot) "TraceTypeQuery1"))
  (if _returnvalue
    (bind (_bblockinghit _binitialoverlap _time _distance _location _impactpoint _normal _impactnormal _physmat _hitactor) (`GameplayStatics.BreakHitResult` _outhit))
    (if (== _hitactor EnemyToShoot)
      (`GameplayStatics.ApplyDamage` _hitactor 10.0 (`self.GetController`) self "/Script/Engine.DamageType"))))

(event `self.ReceiveBeginPlay`
  (`SceneComponent.K2_AttachToComponent` (`self.GunMesh`) (`self.Mesh`) "WeaponSocket" "SnapToTarget" "SnapToTarget" "SnapToTarget" true))

(event `PlayShootFX`
  (bind _gunmesh (`self.GunMesh`))
  (`GameplayStatics.SpawnEmitterAtLocation` "/Game/ExternalContent/MaterialFunctionCollection/ShowcaseAssets/ExampleContent/Effects/P_Pulse_Ring.P_Pulse_Ring" (`SceneComponent.GetSocketLocation` _gunmesh "Socket") (`SceneComponent.GetSocketRotation` _gunmesh "Socket")))

(fn `UserConstructionScript`)