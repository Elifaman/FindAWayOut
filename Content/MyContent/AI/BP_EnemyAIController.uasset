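; Enemy AI controller that runs BT_Enemy and reports sight of the player to its blackboard.
; On BeginPlay it caches player character 0 and writes it to a blackboard key spelled "Ene,y".
; Perception updates filter for the player and set bCanSeePlayer from the first stimulus's success flag.
; When sensing fails, it saves the player's current position as LastSeenLocation and draws a debug sphere there.
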(event `self.ReceiveBeginPlay`
  (bind _returnvalue (`GameplayStatics.GetPlayerCharacter` 0))
  (`|ExecutionSequence`
    (:`then_0`
      (`self.RunBehaviorTree` "/Game/MyContent/AI/BT_Enemy.BT_Enemy"))
    (:`then_1`
      (set `self.Enemy` _returnvalue)
      (`BlackboardComponent.SetValueAsObject` (`AIBlueprintHelperLibrary.GetBlackboard` null) "Ene,y" _returnvalue))))

(event `self.AIPerception.OnPerceptionUpdated`
  (params (UpdatedActors :type "Array of Actor Object Reference (by ref)"))
  (bind _returnvalue (`AIBlueprintHelperLibrary.GetBlackboard` null))
  (bind _returnvalue_2 (`self.K2_GetActorLocation` (`self.Enemy`)))
  (for _array_element UpdatedActors
    (if (== _array_element (`self.Enemy`))
      (bind _info (`AIPerceptionComponent.GetActorsPerception` (`self.AIPerception`) _array_element))
      (bind (_age _expirationage _strength _stimuluslocation _receiverlocation _tag _bsuccessfullysensed) (break `AIStimulus` (`|GetArrayItem` (`.LastSensedStimuli` (break `ActorPerceptionBlueprintInfo` _info)))))
      (`BlackboardComponent.SetValueAsBool` _returnvalue "bCanSeePlayer" _bsuccessfullysensed)
      (if (not _bsuccessfullysensed)
        (`BlackboardComponent.SetValueAsVector` _returnvalue "LastSeenLocation" _returnvalue_2)
        (`KismetSystemLibrary.DrawDebugSphere` _returnvalue_2 100.0 12 (struct :`R` 1.0 :`G` 1.0 :`B` 1.0 :`A` 1.0) 5.0 1.0)))))

(fn `UserConstructionScript`)